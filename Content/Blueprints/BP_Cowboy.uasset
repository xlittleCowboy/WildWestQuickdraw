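; BP_Cowboy is a cowboy that takes Aim and Fire input and exposes a projectile origin for shooting.
; Pressing and releasing each input sets and clears the IsAiming and IsFiring flags.
; Two getter functions return the world location and forward vector of the ProjectileSpawn component as a shot's start point and direction.
; The Blueprint itself spawns no projectiles and has no logic in BeginPlay, Tick or construction.
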(event EventBeginPlay)

(event Collision|EventActorBeginOverlap
  (params (OtherActor :type Actor%20Object%20Reference)))

(event EventTick
  (params (DeltaSeconds :type Float%20%28single-precision%29)))

(event Input|ActionEvents|InputActionAim
  (params (Key :type Key%20Structure :default "None"))
  (:Pressed
    (Variables|Default|SetisAiming true))
  (:Released
    (Variables|Default|SetisAiming false)))

(event Input|ActionEvents|InputActionFire
  (params (Key :type Key%20Structure :default "None"))
  (:Pressed
    (Variables|Default|SetisFiring true))
  (:Released
    (Variables|Default|SetisFiring false)))

(fn ConstructionScript)

(fn GetStartProjectileDirection
  (return (Math|Vector|GetForwardVector (Variables|Default|GetProjectileSpawn))))

(fn GetStartProjectileLocation
  (return (Transformation|GetWorldLocation (Variables|Default|GetProjectileSpawn))))