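; BP_Projectile is a projectile actor that deploys a BP_ForceField where it hits.
; Its Hit event calls SpawnForceField, which uses a DoOnce so only one force field spawns, at the static mesh's world location.
; Getter functions expose the ProjectileMovement and StaticMesh components.
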(event Custom|SpawnForceField
  (Utilities|FlowControl|DoOnce false
    (:Completed
      (Game|SpawnActorfromClass "/Game/Blueprints/BP_ForceField.BP_ForceField_C" (Math|Conversions|ToTransform(Vector) (Transformation|GetWorldLocation (Variables|Default|GetStaticMesh))) "Undefined" 0 0))))

(event Collision|EventHit
  (params (MyComp :type Primitive%20Component%20Object%20Reference) (Other :type Actor%20Object%20Reference) (OtherComp :type Primitive%20Component%20Object%20Reference) (bSelfMoved :type Boolean) (HitLocation :type Vector :default "0, 0, 0") (HitNormal :type Vector :default "0, 0, 0") (NormalImpulse :type Vector :default "0, 0, 0") (Hit :type Hit%20Result%20Structure%20%28by%20ref%29))
  (CallFunction|SpawnForceField))

(fn ConstructionScript)

(fn GetProjectileMovementComponent
  (return (Variables|Default|GetProjectileMovement)))

(fn GetMesh
  (return (Variables|Default|GetStaticMesh)))